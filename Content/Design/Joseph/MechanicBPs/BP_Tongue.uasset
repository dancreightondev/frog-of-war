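; BP_Tongue is a tongue projectile that retracts to its launch point and drags a hit player character with it.
; A custom event records the sphere's location, then after a short delay plays the Comeback timeline, which zeroes projectile velocity and lerps the sphere back.
; A sphere hit starts the retraction immediately and, for a Player_Character, a second timeline lerps its capsule to that location.
; Either timeline destroys the actor on finishing.
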(event OnComponentHit(Sphere)
  (params (HitComponent :type Primitive%20Component%20Object%20Reference) (OtherActor :type Actor%20Object%20Reference) (OtherComp :type Primitive%20Component%20Object%20Reference) (NormalImpulse :type Vector :default "0, 0, 0") (Hit :type Hit%20Result%20Structure%20%28by%20ref%29))
  (Utilities|FlowControl|Sequence
    (:then_0
      (bind _newtrack_0 (Timeline|Comeback Play)
        (:Update
          (Variables|/Script/Engine.MovementComponent|SetVelocity (Variables|Default|GetProjectileMovement) "0, 0, 0")
          (Transformation|SetWorldLocation (Variables|Default|GetSphere) (Math|Vector|Lerp(Vector) (Transformation|GetWorldLocation (Variables|Default|GetSphere)) (stale Custom|CustomEvent _output_get) _newtrack_0) false false))
        (:Finished
          (Actor|DestroyActor))))
    (:then_1
      (bind _asplayer_character (Utilities|Casting|CastToPlayer_Character OtherActor))
      (bind _newtrack_0_2 (Timeline|Timeline_1 Play)
        (:Update
          (Transformation|SetWorldLocation (Variables|/Script/Engine.Character|GetCapsuleComponent _asplayer_character) (Math|Vector|Lerp(Vector) (Transformation|GetWorldLocation (Variables|/Script/Engine.Character|GetCapsuleComponent _asplayer_character)) (Variables|Default|GetLocation) _newtrack_0_2) false false))
        (:Finished
          (Actor|DestroyActor))))))

(event Custom|CustomEvent
  (bind _sphere (Variables|Default|GetSphere))
  (bind _returnvalue (Transformation|GetWorldLocation _sphere))
  (bind _output_get (Variables|Default|SetLocation _returnvalue))
  (Utilities|FlowControl|Delay 0.2)
  (bind _newtrack_0 (Timeline|Comeback Play)
    (:Update
      (Variables|/Script/Engine.MovementComponent|SetVelocity (Variables|Default|GetProjectileMovement) "0, 0, 0")
      (Transformation|SetWorldLocation (Variables|Default|GetSphere) (Math|Vector|Lerp(Vector) _returnvalue _output_get _newtrack_0) false false))
    (:Finished
      (Actor|DestroyActor))))

(fn ConstructionScript)