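; Base Blueprint for wild card pickups that modify the player character's health and movement speed.
; When a Player_Character overlaps its Box, it applies those values through WildCardUpdate, registers its colour in the player's inventory, plays a sound and destroys itself.
; If the inventory's third wild card slot is already filled, it only prints a "WildCards Full" message.
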(event OnComponentBeginOverlap(Box)
  (params (OverlappedComponent :type Primitive%20Component%20Object%20Reference) (OtherActor :type Actor%20Object%20Reference) (OtherComp :type Primitive%20Component%20Object%20Reference) (OtherBodyIndex :type Integer) (bFromSweep :type Boolean) (SweepResult :type Hit%20Result%20Structure%20%28by%20ref%29))
  (bind _asplayer_character (Utilities|Casting|CastToPlayer_Character OtherActor))
  (if (Variables|/Game/Inventory/Inventory.Inventory_C|GetWildCardSlot3Filled? (Variables|/Game/Player_Character.Player_Character_C|GetInventoryRef _asplayer_character))
    (Development|PrintString "WildCards Full")
    (else
      (Default|WildCardUpdate _asplayer_character (Variables|Default|GetHealth) (Variables|Default|GetMovement%20Speed))
      (Default|WildCardPickUp (Variables|/Game/Player_Character.Player_Character_C|GetInventoryRef _asplayer_character) (Variables|Default|GetWildCardColour))
      (Audio|PlaySound2D 0 1.0 1.0 0.0 0 0)
      (Actor|DestroyActor))))

(event EventBeginPlay)

(event Collision|EventActorBeginOverlap
  (params (OtherActor :type Actor%20Object%20Reference)))

(event EventTick
  (params (DeltaSeconds :type Float%20%28single-precision%29)))

(fn ConstructionScript)