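; Parent armour pickup actor that gives armour to the player character overlapping its box, with support for up to four local players.
; A MultiGate started at the player controller ID selects that player's inventory reference.
; If that inventory's hold is full it prints a message and resets the gate; otherwise it notifies the character and inventory, passing the armour picture, plays a sound and destroys itself.
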(event OnComponentBeginOverlap(Box)
  (params (OverlappedComponent :type Primitive%20Component%20Object%20Reference) (OtherActor :type Actor%20Object%20Reference) (OtherComp :type Primitive%20Component%20Object%20Reference) (OtherBodyIndex :type Integer) (bFromSweep :type Boolean) (SweepResult :type Hit%20Result%20Structure%20%28by%20ref%29))
  (bind _asplayer_character (Utilities|Casting|CastToPlayer_Character OtherActor))
  (Variables|Default|SetPlayer%20Ref _asplayer_character)
  (bind _asplayer_controller (Utilities|Casting|CastToPlayerController (Pawn|GetController (Variables|Default|GetPlayer%20Ref))))
  (Utilities|FlowControl|MultiGate false false (Class|GameplayStatics|GetPlayerControllerID _asplayer_controller)
    (:Out%200
      (if (Variables|/Game/Blueprints/UMG/Widgets/Inventory/Player1HUD.Player1HUD_C|GetHoldFull? (Variables|/Game/Player_Character.Player_Character_C|GetInventory1Ref (Variables|Default|GetPlayer%20Ref)))
        (Development|PrintString "Armour Full")
        (CallFunction|ResetArmour)
        (else
          (Default|ArmourPickUp (Variables|Default|GetPlayer%20Ref))
          (Default|ArmourPickUp (Variables|/Game/Player_Character.Player_Character_C|GetInventory1Ref (Variables|Default|GetPlayer%20Ref)) "NewEnumerator1" (Variables|Default|GetArmourColour))
          (Audio|PlaySound2D 0 1.0 1.0 0.0 0 0)
          (Actor|DestroyActor))))
    (:Out%201
      (if (Variables|/Game/Blueprints/UMG/Widgets/Inventory/Player2HUD.Player2HUD_C|GetHoldFull? (Variables|/Game/Player_Character.Player_Character_C|GetInventory2Ref (Variables|Default|GetPlayer%20Ref)))
        (Development|PrintString "Armour Full")
        (CallFunction|ResetArmour)
        (else
          (Default|ArmourPickUp (Variables|Default|GetPlayer%20Ref))
          (Default|ArmourPickUp (Variables|/Game/Player_Character.Player_Character_C|GetInventory2Ref (Variables|Default|GetPlayer%20Ref)) "NewEnumerator1" (Variables|Default|GetArmourColour))
          (Audio|PlaySound2D 0 1.0 1.0 0.0 0 0)
          (Actor|DestroyActor))))
    (:Out%202
      (if (Variables|/Game/Blueprints/UMG/Widgets/Inventory/Player3HUD.Player3HUD_C|GetHoldFull? (Variables|/Game/Player_Character.Player_Character_C|GetInventory3Ref (Variables|Default|GetPlayer%20Ref)))
        (Development|PrintString "Armour Full")
        (CallFunction|ResetArmour)
        (else
          (Default|ArmourPickUp (Variables|Default|GetPlayer%20Ref))
          (Default|ArmourPickUp (Variables|/Game/Player_Character.Player_Character_C|GetInventory3Ref (Variables|Default|GetPlayer%20Ref)) "NewEnumerator1" (Variables|Default|GetArmourColour))
          (Audio|PlaySound2D 0 1.0 1.0 0.0 0 0)
          (Actor|DestroyActor))))
    (:Out%203
      (if (Variables|/Game/Blueprints/UMG/Widgets/Inventory/Player4HUD.Player4HUD_C|GetHoldFull? (Variables|/Game/Player_Character.Player_Character_C|GetInventory4Ref (Variables|Default|GetPlayer%20Ref)))
        (Development|PrintString "Armour Full")
        (CallFunction|ResetArmour)
        (else
          (Default|ArmourPickUp (Variables|Default|GetPlayer%20Ref))
          (Default|ArmourPickUp (Variables|/Game/Player_Character.Player_Character_C|GetInventory4Ref (Variables|Default|GetPlayer%20Ref)) "NewEnumerator1" (Variables|Default|GetArmourColour))
          (Audio|PlaySound2D 0 1.0 1.0 0.0 0 0)
          (Actor|DestroyActor))))))

(event Custom|Reset%20Armour
  (Utilities|FlowControl|MultiGate false false (Class|GameplayStatics|GetPlayerControllerID (stale OnComponentBeginOverlap(Box) _asplayer_controller))) ; enters at Reset
)

(event EventBeginPlay)

(event Collision|EventActorBeginOverlap
  (params (OtherActor :type Actor%20Object%20Reference)))

(event EventTick
  (params (DeltaSeconds :type Float%20%28single-precision%29)))

(fn ConstructionScript)